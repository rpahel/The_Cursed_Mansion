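; Pushable actor that a character with a PushComponent can interact with to start pushing it.
; Its construction script adds an arrow for each PushTransforms entry as a grab position.
; On interaction it picks the nearest position within push range in 2D, then traces for standing room, walkable floor and blocking walls.
; On success it teleports and orients the character and calls BeginPush; failures print debug reasons.
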(event `/Game/MouvableItems/Interact_Interface.OnInteracted`
  (params (Player :type "/Game/FirstPersonBP/Blueprints/FirstPersonCharacter Object Reference"))
  (`self.HandleInteraction` Player))

(fn `FinClosestPushTransformIndex`
  (params (CharacterLocation :type "Vector2D Structure") (PushRange :type "Float (double-precision)"))
  (returns (BestIndex :type Integer))
  (locals (CurentTransformIndex :type Integer) (CurrentDistanceSq :type "Float (double-precision)" :default 0.0) (ClosestTransformIndex :type Integer :default -1) (ClostestDistanceSq :type "Float (double-precision)"))
  (for (_array_element _array_index) (`self.PushTransforms`)
    ;[1 0.1939 0.533] Get The World Location
    (set `local.CurentTransformIndex` _array_index)
    ;[1 0.5164 0.1242] ...To the range value...
    (bind _output_get (set `local.CurrentDistanceSq` (`KismetMathLibrary.DistanceSquared2D` (`KismetMathLibrary.Conv_VectorToVector2D` (`KismetMathLibrary.TransformLocation` (`self.GetTransform`) (.location _array_element))) (`local.CharacterLocation`))))
    (if (< _output_get (`KismetMathLibrary.Square` (`local.PushRange`)))
      ;[0.9566 1 0.08689] ...Then to the last clostest Value (and change it if it's close)
      (if (or (< (`local.CurrentDistanceSq`) (`local.ClostestDistanceSq`)) (< (`local.ClosestTransformIndex`) 0))
        (set `local.ClosestTransformIndex` (`local.CurentTransformIndex`))
        (set `local.ClostestDistanceSq` (`local.CurrentDistanceSq`))
        (`KismetSystemLibrary.PrintString` (`KismetStringLibrary.Concat_StrStr` "Index " (`KismetStringLibrary.Conv_IntToString` (`local.CurentTransformIndex`)) " is at  : " (`KismetStringLibrary.Conv_DoubleToString` (`local.CurrentDistanceSq`))) true true (struct :`R` 0.045745 :`B` 1.0 :`A` 1.0) 5.0))
      (else
        (`KismetSystemLibrary.PrintString` (`KismetStringLibrary.Concat_StrStr` "Index " (`KismetStringLibrary.Conv_IntToString` (`local.CurentTransformIndex`)) " is at  : " (`KismetStringLibrary.Conv_DoubleToString` (`local.CurrentDistanceSq`))) true true (struct :`G` 0.66 :`B` 1.0 :`A` 1.0) 5.0))))
  (`KismetSystemLibrary.PrintString` (`KismetStringLibrary.Concat_StrStr` "Index num " (`KismetStringLibrary.Conv_IntToString` (`local.ClosestTransformIndex`)) " Is Retun") true true (struct :`R` 1.0 :`B` 0.142179 :`A` 1.0))
  (return (`local.ClosestTransformIndex`)))

(fn `HandleInteraction`
  (params (Character :type "Character Object Reference"))
  (locals (PushComponent :type "/Game/MouvableItems/PushComponent Object Reference") (CharacterPrevTransform :type "Transform Structure") (CharacterNewTransform :type "Transform Structure"))
  (bind _characternewtransform_location (`KismetMathLibrary.BreakTransform` (`local.CharacterNewTransform`)))
  (bind (_characternewtransform_location_2 _characternewtransform_rotation) (`KismetMathLibrary.BreakTransform` (`local.CharacterNewTransform`)))
  (bind (_characternewtransform_location_3 _characternewtransform_rotation_2 _characternewtransform_scale) (`KismetMathLibrary.BreakTransform` (`local.CharacterNewTransform`)))
  (bind _capsulecomponent (`Character.CapsuleComponent` (`local.Character`)))
  ;[0.8612 1 0.1332] Check If Exist
  (`/Engine/EditorBlueprintResources/StandardMacros.IsValid` Character
    (:`Is Valid`
      (bind _output_get (set `local.PushComponent` (`self.GetComponentByClass` Character "/Game/MouvableItems/PushComponent.PushComponent_C")))
      (`/Engine/EditorBlueprintResources/StandardMacros.IsValid` _output_get
        (:`Is Valid`
          ;[0.425 1 0.1706] check the closest point
          (bind _bestindex (`self.FinClosestPushTransformIndex` (`KismetMathLibrary.Conv_VectorToVector2D` (`self.K2_GetActorLocation` (`local.Character`))) (`/Game/MouvableItems/PushComponent.PushRange` (`local.PushComponent`))))
          (if (>= _bestindex 0)
            (bind (_returnvalue_location _returnvalue_rotation _returnvalue_scale) (`KismetMathLibrary.BreakTransform` (`KismetMathLibrary.ComposeTransforms` (`|GetArrayItem` (`self.PushTransforms`) _bestindex) (`self.GetTransform`))))
            ;[0.3166 1 0.5721] set the red point to the hips in order to teleport him after
            (bind _output_get_2 (set `local.CharacterNewTransform` (`KismetMathLibrary.MakeTransform` (+ _returnvalue_location (`KismetMathLibrary.MakeVector` 0.0 0.0 (`CapsuleComponent.GetScaledCapsuleHalfHeight` (`Character.CapsuleComponent` (`local.Character`))))) _returnvalue_rotation _returnvalue_scale)))
            ;[0.4427 1 0.9191] Verify if we have enought space to push it
            (`KismetSystemLibrary.DrawDebugSphere` (.location _output_get_2) 20.0 12 (struct :`R` 1.0 :`B` 0.023145 :`A` 1.0) 2.0 1.0)
            (bind _outhit (`KismetSystemLibrary.CapsuleTraceSingle` :`Start` (+ _characternewtransform_location_3 (0.0 0.0 70.0)) :`End` (+ _characternewtransform_scale (0.0 0.0 100.0)) :`Radius` (`CapsuleComponent.GetScaledCapsuleRadius` _capsulecomponent) :`HalfHeight` (`CapsuleComponent.GetScaledCapsuleHalfHeight` _capsulecomponent) :`TraceChannel` "TraceTypeQuery1" :`DrawDebugType` "ForDuration"))
            (bind (_bblockinghit _binitialoverlap _time _distance _location _impactpoint _normal _impactnormal) (`GameplayStatics.BreakHitResult` _outhit))
            (if (not _binitialoverlap)
              (if (< (`CharacterMovementComponent.K2_GetWalkableFloorZ` (`Character.CharacterMovement` (`local.Character`))) (.z _impactnormal))
                (bind (_outhit_2 _returnvalue) (`KismetSystemLibrary.LineTraceSingle` (`self.K2_GetActorLocation`) _characternewtransform_location "TraceTypeQuery1" false (`|MakeArray` (`local.Character`) :!type "Actor Object Reference") "None" true (struct :`R` 1.0 :`A` 1.0) (struct :`G` 1.0 :`A` 1.0) 2.0))
                (if (not _returnvalue)
                  (`self.K2_SetActorTransform` (`local.Character`) (`local.CharacterNewTransform`) false true)
                  (`Controller.SetControlRotation` (`GameplayStatics.GetPlayerController` 0) _characternewtransform_rotation)
                  (`/Game/MouvableItems/PushComponent.BeginPush` (`local.PushComponent`) self)
                  (else
                    (`self.PushFailedInfo` "Wall in between character and object")))
                (else
                  (`self.PushFailedInfo` "Floor not walkable")))
              (else
                (`self.PushFailedInfo` "No room to stand")))
            (else
              (`self.PushFailedInfo` "No push transform found"))))
        (:`Is Not Valid`
          (`self.PushFailedInfo` "Character doesn't have a push component"))))
    (:`Is Not Valid`
      (`self.PushFailedInfo` "Character is Invalid"))))

(fn `UserConstructionScript`
  (for _array_element (`self.PushTransforms`)
    (`AddComponent|NODE_AddArrowComponent-0` :`RelativeTransform` _array_element)))